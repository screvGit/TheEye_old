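; Double door actor that swings two door meshes open or closed when its Interact function is called.
; A single timeline plays forward or in reverse, lerping each door's relative rotation between its closed and open rotations along the shortest path.
; Separate open and close durations set the timeline play rate.
; IsOpen flips only when the timeline finishes, so interacting mid-swing does not change direction.
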(event Custom|Open%20Door
  (bind _door_track (Timeline|Open%20Door%20T Play)
    (:Update
      (Transformation|SetRelativeRotation (Variables|Default|GetDoor1) (Math|Rotator|Lerp(Rotator) (Variables|Default|GetD1ClosePosition) (Variables|Default|GetD1OpenPosition) _door_track true) false false)
      (Transformation|SetRelativeRotation (Variables|Default|GetDoor%202) (Math|Rotator|Lerp(Rotator) (Variables|Default|GetD2ClosePosition) (Variables|Default|GetD2OpenPosition) _door_track true) false false))
    (:Finished
      (Variables|Default|SetIsOpen (not (Variables|Default|GetIsOpen))))))

(event Custom|Close%20Door
  (bind _door_track (Timeline|Open%20Door%20T Reverse)
    (:Update
      (Transformation|SetRelativeRotation (Variables|Default|GetDoor1) (Math|Rotator|Lerp(Rotator) (Variables|Default|GetD1ClosePosition) (Variables|Default|GetD1OpenPosition) _door_track true) false false)
      (Transformation|SetRelativeRotation (Variables|Default|GetDoor%202) (Math|Rotator|Lerp(Rotator) (Variables|Default|GetD2ClosePosition) (Variables|Default|GetD2OpenPosition) _door_track true) false false))
    (:Finished
      (Variables|Default|SetIsOpen (not (Variables|Default|GetIsOpen))))))

(event EventBeginPlay)

(event Collision|EventActorBeginOverlap
  (params (OtherActor :type Actor%20Object%20Reference)))

(event EventTick
  (params (DeltaSeconds :type Float%20%28single-precision%29)))

(fn ConstructionScript)

(fn Interact
  (params (Interactor :type Character%20Object%20Reference))
  (bind _open_door_t (Variables|Default|GetOpen%20Door%20T))
  (if (not (Variables|Default|GetIsOpen))
    (Components|Timeline|SetPlayRate _open_door_t (/ 1.0 (Variables|Default|GetTimeToOpen%28s%29)))
    (CallFunction|OpenDoor)
    (else
      (Components|Timeline|SetPlayRate _open_door_t (/ 1.0 (Variables|Default|GetTimeToClose%28s%29)))
      (CallFunction|CloseDoor)))
  (return true))